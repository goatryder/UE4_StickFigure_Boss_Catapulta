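; BP_Checkpoint is a single-use flag checkpoint that saves the player character's respawn location in BP_MyGameMode.
; Overlapping its box marks it used, stores the offset location, swaps the sprite to a white flag, plays a sound and notifies BP_HUD.
; A checkpoint flagged as last also makes the GameMode check level completion.
; The construction script sizes and raises the box and shows a green flag for the last checkpoint.
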(event OnComponentBeginOverlap(Box)
  (params (OverlappedComponent :type Primitive%20Component%20Object%20Reference) (OtherActor :type Actor%20Object%20Reference) (OtherComp :type Primitive%20Component%20Object%20Reference) (OtherBodyIndex :type Integer) (bFromSweep :type Boolean) (SweepResult :type Hit%20Result%20Structure%20%28by%20ref%29))
  (bind _gamemode (Variables|Default|GetGameMode))
  (if (not (Variables|Default|GetbIsUsed))
    (bind _asbp_my_character (Utilities|Casting|CastToBP_MyCharacter OtherActor))
    (Utilities|IsValid (Variables|Default|GetGameMode)
      (:Is%20Valid
        (Utilities|FlowControl|Sequence
          (:then_0
            (Variables|Default|SetbIsUsed true))
          (:then_1
            ;[1 1 1] Set GameMode Last checkpoint
            (Variables|/Game/Blueprints/BP_MyGameMode.BP_MyGameMode_C|SetCharacterLastCheckPoint _gamemode (+ (Variables|Default|GetSpawnPointOffset) (Transformation|GetActorLocation)))
            (bind _output_get (Variables|/Game/Blueprints/BP_MyGameMode.BP_MyGameMode_C|SetbLastCheckpointReached _gamemode (Variables|Default|GetbIsLast)))
            (if _output_get
              (Default|CheckCurrentLevelComplete _gamemode)
              (Development|PrintString "GM LAST CHECKPOINT REACHED" true true "(R=1.000000,G=0.000000,B=0.000000,A=1.000000)" 5.0)))
          (:then_2
            (CallFunction|UsedFX))
          (:then_3
            ;[1 1 1] HUD Checkpoint reached msg
            (bind _asplayer_controller (Utilities|Casting|CastToPlayerController (Pawn|GetController _asbp_my_character)))
            (bind _asbp_hud (Utilities|Casting|CastToBP_HUD (HUD|GetHUD _asplayer_controller)))
            (Default|CheckpointReached _asbp_hud)))))))

(event Custom|UsedFX
  (Rendering|Components|Sprite|SetSprite (Variables|Default|GetPaperSprite) "/Game/2DAssets/Flags/FlagWhite_Sprite.FlagWhite_Sprite")
  (Audio|PlaySound2D "/Game/Sound/PaperSheetShortCue.PaperSheetShortCue" 1.0 1.0 0.0 0 0))

(event EventBeginPlay
  (bind _asbp_my_game_mode (Utilities|Casting|CastToBP_MyGameMode (Game|GetGameMode)))
  (Variables|Default|SetGameMode _asbp_my_game_mode))

(fn ConstructionScript
  (bind _box (Variables|Default|GetBox))
  (Components|Box|SetBoxExtent _box (Variables|Default|GetCollisionBoxExtend) true)
  (Transformation|AddLocalOffset _box (Math|Vector|MakeVector 0.0 0.0 (.z (Variables|Default|GetCollisionBoxExtend))) false false)
  (if (Variables|Default|GetbIsLast)
    (Rendering|Components|Sprite|SetSprite (Variables|Default|GetPaperSprite) "/Game/2DAssets/Flags/FlagGreen_Sprite.FlagGreen_Sprite")))