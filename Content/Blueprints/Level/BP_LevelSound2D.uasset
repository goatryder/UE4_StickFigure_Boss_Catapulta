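; BP_LevelSound2D is a placeable level sound zone that plays an assigned 2D sound while BP_MyCharacter is inside its box.
; The construction script applies the box extent and sound, and PlayOnStart triggers playback there and on BeginPlay.
; Box overlaps set CanPlay and fade the audio in or out over one second.
; When playback finishes, it fades in again if LoopSound and CanPlay are set.
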(event OnComponentBeginOverlap(Box)
  (params (OverlappedComponent :type Primitive%20Component%20Object%20Reference) (OtherActor :type Actor%20Object%20Reference) (OtherComp :type Primitive%20Component%20Object%20Reference) (OtherBodyIndex :type Integer) (bFromSweep :type Boolean) (SweepResult :type Hit%20Result%20Structure%20%28by%20ref%29))
  (Utilities|Casting|CastToBP_MyCharacter OtherActor)
  (Variables|Default|SetbCanPlay true)
  (if (not (Audio|Components|Audio|IsPlaying (Variables|Default|GetAudio)))
    (Audio|Components|Audio|FadeIn (Variables|Default|GetAudio) 1.0 1.0 0.0 "Linear" :!class /Script/Engine.AudioComponent)))

(event OnComponentEndOverlap(Box)
  (params (OverlappedComponent :type Primitive%20Component%20Object%20Reference) (OtherActor :type Actor%20Object%20Reference) (OtherComp :type Primitive%20Component%20Object%20Reference) (OtherBodyIndex :type Integer))
  (Utilities|Casting|CastToBP_MyCharacter OtherActor)
  (Variables|Default|SetbCanPlay false)
  (if (Audio|Components|Audio|IsPlaying (Variables|Default|GetAudio))
    (Audio|Components|Audio|FadeOut (Variables|Default|GetAudio) 1.0 0.0 "Linear" :!class /Script/Engine.AudioComponent)))

(event OnAudioFinished(Audio)
  ;[1 1 1] Handle Play Loop
  (if (and (Variables|Default|GetbLoopSound) (Variables|Default|GetbCanPlay))
    (Audio|Components|Audio|FadeIn (Variables|Default|GetAudio) 1.0 1.0 0.0 "Linear" :!class /Script/Engine.AudioComponent)))

(event EventBeginPlay
  (if (Variables|Default|GetbPlayOnStart)
    (Audio|Components|Audio|FadeIn (Variables|Default|GetAudio) 1.0 1.0 0.0 "Linear" :!class /Script/Engine.AudioComponent)))

(fn ConstructionScript
  (bind _audio (Variables|Default|GetAudio))
  (Components|Box|SetBoxExtent (Variables|Default|GetBox) (Variables|Default|GetBoxExtend) true)
  (Audio|Components|Audio|SetSound _audio (Variables|Default|GetSound2D))
  (if (Variables|Default|GetbPlayOnStart)
    (Audio|Components|Audio|FadeIn _audio 1.0 1.0 0.0 "Linear" :!class /Script/Engine.AudioComponent)
    (Variables|Default|SetbCanPlay true)))