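; Paper2D enemy on the XZ plane that patrols, shoots projectiles and damages BP_MyCharacter on overlap.
; Tick moves it between two points or random points within a radius, optionally flipping sprite and muzzle to face travel.
; Firing loops through a randomised cooldown macro with a brief sprite swap.
; Armour must be depleted before health takes damage, with dispatchers and empty hooks for armour break and death; wavy-motion timeline is unconnected.
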(event Custom|StartFire
  ;[1 1 1] fire
  (if (Variables|Default|GetbCanFire)
    (CallFunction|Fire)
    (CallFunction|FireAnim)
    (Utilities|FireCooldown
      (:out
        (CallFunction|StartFire)))))

(event Custom|StopFire
  ;[1 1 1] fire
  (Variables|Default|SetbCanFire false))

(event Custom|DamageHealth
  (params (DamageHealthVal :type Integer))
  ;[1 1 1] Receive health damage
  (if (<= (Variables|Default|GetArmour) 0)
    (bind _output_get (Variables|Default|SetHealth (- (Variables|Default|GetHealth) DamageHealthVal)))
    (Default|CallRecieveHealthDamage DamageHealthVal)
    (if (<= _output_get 0)
      (Default|CallDied)
      (CallFunction|OnDeath)
      (Effects|SpawnEmitteratLocation "/Game/Effects/KillEnemy.KillEnemy" (Transformation|GetActorLocation))
      (Actor|DestroyActor))))

(event Custom|FireAnim
  ;[1 1 1] fire
  (Rendering|Components|Sprite|SetSprite (Variables|Default|GetSprite) (Variables|Default|GetEnemySpriteFire))
  (Utilities|FlowControl|Delay (Variables|Default|GetFireAnimTime))
  (Rendering|Components|Sprite|SetSprite (Variables|Default|GetSprite) (Variables|Default|GetEnemySprite)))

(event Custom|TestChangeFacing
  ;[1 1 1] test
  (Utilities|FlowControl|Delay 2.0)
  (CallFunction|SetFacing (not (Variables|Default|GetFaceLeft)))
  (CallFunction|TestChangeFacing))

(event Custom|Fire
  ;[1 1 1] fire
  (Game|SpawnActorfromClass "/Game/Blueprints/Projectiles/EnemyProjectileDefult.EnemyProjectileDefult_C" (Transformation|GetWorldTransform (Variables|Default|GetProjectileSpawnPoint)) "AdjustIfPossibleButDontSpawnIfColliding" 0 0))

(event Custom|DamageArmour
  (params (DamageArmourVal :type Integer))
  ;[1 1 1] Receive Armour Damage
  ;;[1 1 1] Event Should not fire if armour is already zero or less
  (if (> (Variables|Default|GetArmour) 0)
    (Variables|Default|SetArmour (- (Variables|Default|GetArmour) DamageArmourVal))
    (Default|CallRecieveArmourDamage DamageArmourVal)
    (if (< (Variables|Default|GetArmour) 1)
      (Default|CallArmourIsDestroyed)
      (CallFunction|ArmourDestroyed))))

(event Custom|OnDeath)

(event Custom|ArmourDestroyed)

(event EventBeginPlay
  (CallFunction|FirefromStartHandle)
  (CallFunction|SetInitProjectileSpawnTransform)
  (CallFunction|InitPatrol))

(event EventTick
  (params (DeltaSeconds :type Float%20%28single-precision%29))
  (if (Variables|Patrol|GetbCanPatrol)
    (CallFunction|MovetoPatrolPoint DeltaSeconds)
    (if (CallFunction|IsPatrolPointReached)
      (CallFunction|SelectPatrolPoint))))

(event Collision|EventActorBeginOverlap
  (params (OtherActor :type Actor%20Object%20Reference))
  ;[1 1 1] overlap
  (bind _asbp_my_character (Utilities|Casting|CastToBP_MyCharacter OtherActor))
  (Default|Damage _asbp_my_character 1))

(fn ConstructionScript
  (bind _returnvalue (Transformation|GetActorLocation))
  (bind _projectilemovement1 (Variables|Default|GetProjectileMovement1))
  (bind _projectilespawnpoint (Variables|Default|GetProjectileSpawnPoint))
  (bind (_x _y _z) (Math|Vector|BreakVector _returnvalue))
  (bind _relativelocation (Variables|/Script/Engine.SceneComponent|GetRelativeLocation _projectilespawnpoint))
  (bind _returnvalue_2 (AddComponent|AddPaperSpriteComponent false))
  (Variables|Default|SetSprite _returnvalue_2)
  (Rendering|Components|Sprite|SetSprite _returnvalue_2 (Variables|Default|GetEnemySprite))
  (if (Variables|Default|GetLiveForever)
    (Actor|SetLifeSpan 0.0))
  (if (Variables|Patrol|GetbCanPatrol)
    (Variables|/Script/Engine.ProjectileMovementComponent|SetInitialSpeed _projectilemovement1 5e+02)
    (else
      (Variables|/Script/Engine.ProjectileMovementComponent|SetInitialSpeed _projectilemovement1 0.0)))
  (if (Variables|Default|GetHasWavyMotion)
    (Variables|Default|SetInternalWaveAmount (Variables|Default|GetWaveAmount))
    (else
      (Variables|Default|SetInternalWaveAmount 0.0)))
  (if (Variables|Default|GetFaceLeft)
    (Transformation|AddRelativeRotation (Variables|Default|GetSprite) (Math|Rotator|MakeRotator 0.0 0.0 1.8e+02) false false)
    (Transformation|SetRelativeTransform _projectilespawnpoint (Math|Transform|MakeTransform (Math|Vector|MakeVector (* (.x _relativelocation) -1.0) (.y _relativelocation) (.z _relativelocation)) "0.000000,180.000000, 0" "1,1,1") false false)
    (Transformation|SetActorLocation (Math|Vector|MakeVector _x 0.0 _z) false false)))

(fn SetFacing
  (params (bFaceLeft :type Boolean))
  (bind _returnvalue (Transformation|GetActorLocation))
  (bind _returnvalue_2 (Transformation|GetActorLocation))
  (bind _initprojectilespawntransofrm (Variables|Default|GetInitProjectileSpawnTransofrm))
  (bind (_x _y _z) (Math|Vector|BreakVector _returnvalue))
  (bind (_x_2 _y_2 _z_2) (Math|Vector|BreakVector _returnvalue_2))
  (bind _output_get (Variables|Default|SetFaceLeft bFaceLeft))
  (if _output_get
    ;[1 1 1] left
    (Transformation|SetRelativeRotation (Variables|Default|GetSprite) "0,180.000000, 0" false false)
    (Transformation|SetRelativeTransform (Variables|Default|GetProjectileSpawnPoint) (Math|Transform|MakeTransform (Math|Vector|MakeVector (* (.x (.location _initprojectilespawntransofrm)) -1.0) (.y (.location _initprojectilespawntransofrm)) (.z (.location _initprojectilespawntransofrm))) "0.000000,180.000000, 0" "1,1,1") false false)
    (Transformation|SetActorLocation (Math|Vector|MakeVector _x 0.0 _z) false false)
    (else
      ;[1 1 1] right
      (Transformation|SetRelativeRotation (Variables|Default|GetSprite) "0, 0, 0" false false)
      (Transformation|SetRelativeTransform (Variables|Default|GetProjectileSpawnPoint) (Math|Transform|MakeTransform (.location (Variables|Default|GetInitProjectileSpawnTransofrm)) "0, 0, 0" "1,1,1") false false)
      (Transformation|SetActorLocation (Math|Vector|MakeVector _x_2 0.0 _z_2) false false))))

(fn InitPatrol
  (bind _returnvalue (Transformation|GetActorLocation))
  (Utilities|FlowControl|Sequence
    (:then_0
      (Variables|Patrol|SetInitialLocation _returnvalue)
      (Variables|Patrol|SetLastPatrolPoint _returnvalue)
      (if (Variables|Patrol|GetbPatrolInRandomXZRadius)
        (Variables|Patrol|SetPatrolPoint (CallFunction|GetRandomPatrolPointXZ))
        (else
          (Variables|Patrol|SetPatrolPoint (+ _returnvalue (Variables|Patrol|GetPatrolToRelative))))))
    (:then_1
      (CallFunction|SetNewDirection)
      (if (Variables|Patrol|GetbChangeFacingToDirection)
        (CallFunction|SetFacingbyDirection)))))

(fn SetNewDirection
  (Variables|Patrol|SetDirection (Math|Vector|Normalize (- (Variables|Patrol|GetPatrolPoint) (Variables|Patrol|GetLastPatrolPoint))))
  (return))

(fn MovetoPatrolPoint
  (params (DeltaTime :type Float%20%28single-precision%29))
  (bind _returnvalue (Transformation|GetActorLocation))
  (Utilities|FlowControl|Sequence
    (:then_0
      (Transformation|SetActorLocation (+ (* (Variables|Patrol|GetDirection) (* DeltaTime (Variables|Patrol|GetPatrolSpeed))) (Transformation|GetActorLocation)) false false))
    (:then_1
      ;[1 1 1] Draw debug
      (Rendering|Debug|DrawDebugSphere (Variables|Patrol|GetPatrolPoint) 4e+01 12 "(R=0.000000,G=1.000000,B=0.066276,A=1.000000)" 0.0)
      (Rendering|Debug|DrawDebugArrow _returnvalue (+ _returnvalue (* (Variables|Patrol|GetDirection) 2e+02)) 0.0 "(R=0.157399,G=1.000000,B=0.000000,A=1.000000)" 0.0 0.0))))

(fn SelectPatrolPoint
  (Utilities|FlowControl|Sequence
    (:then_0
      (if (Variables|Patrol|GetbPatrolInRandomXZRadius)
        (Variables|Patrol|SetLastPatrolPoint (Variables|Patrol|GetPatrolPoint))
        (Variables|Patrol|SetPatrolPoint (CallFunction|GetRandomPatrolPointXZ))
        (else
          (LocalVariables|SetTempPatrolPoint (Variables|Patrol|GetLastPatrolPoint))
          (Variables|Patrol|SetLastPatrolPoint (Variables|Patrol|GetPatrolPoint))
          (Variables|Patrol|SetPatrolPoint (LocalVariables|GetTempPatrolPoint)))))
    (:then_1
      (CallFunction|SetNewDirection)
      (if (Variables|Patrol|GetbChangeFacingToDirection)
        (CallFunction|SetFacingbyDirection)))))

(fn IsPatrolPointReached
  (return (<= (Math|Vector|Distance(Vector) (Transformation|GetActorLocation) (Variables|Patrol|GetPatrolPoint)) (Variables|Patrol|GetReachPointTreshold))))

(fn GetRandomPatrolPointXZ
  (bind _initiallocation (Variables|Patrol|GetInitialLocation))
  (LocalVariables|SetTheta (Math|Float|MultiplybyPi (* (Math|Random|RandomFloat) 2.0)))
  (LocalVariables|SetRandRadius (Math|Random|RandomFloatinRange 0.0 (Variables|Patrol|GetPatrolRandomRadius)))
  (return (Math|Vector|MakeVector (+ (* (LocalVariables|GetRandRadius) (Math|Trig|Cos(Radians) (LocalVariables|GetTheta))) (.x _initiallocation)) (.y _initiallocation) (+ (.z _initiallocation) (* (Math|Trig|Sin(Radians) (LocalVariables|GetTheta)) (LocalVariables|GetRandRadius))))))

(fn SetFacingbyDirection
  (CallFunction|SetFacing (> (Math|Vector|DotProduct (Math|Vector|CrossProduct (Variables|Patrol|GetDirection) "0.000000,0.000000,1.000000") "0,1.000000, 0") 0.0))
  (return))

(fn FirefromStartHandle
  (if (Variables|Default|GetbCanFire)
    (CallFunction|StartFire)
    (Variables|Default|SetFireRate (Variables|Default|GetFireRateMax))))

(fn SetInitProjectileSpawnTransform
  (Variables|Default|SetInitProjectileSpawnTransofrm (Transformation|GetRelativeTransform (Variables|Default|GetProjectileSpawnPoint))))