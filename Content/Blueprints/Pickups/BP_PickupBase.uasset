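; Base pickup actor that reacts when BP_MyCharacter overlaps its collision, playing a sound and fading out before destroying itself.
; The overlap calls PickupFX, then the empty OnPicked event, a hook for child pickups to apply their effect to the character.
; PlayPickupAnim toggles a gate on Tick, which lowers the Paper2D sprite's alpha linearly over PickupAnimTime, then destroys the actor.
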(event OnComponentBeginOverlap(PickupCollision)
  (params (OverlappedComponent :type Primitive%20Component%20Object%20Reference) (OtherActor :type Actor%20Object%20Reference) (OtherComp :type Primitive%20Component%20Object%20Reference) (OtherBodyIndex :type Integer) (bFromSweep :type Boolean) (SweepResult :type Hit%20Result%20Structure%20%28by%20ref%29))
  ;[1 1 1] Overlap
  (bind _asmy_character (Utilities|Casting|CastToBP_MyCharacter OtherActor))
  (CallFunction|PickupFX)
  (CallFunction|OnPicked _asmy_character))

(event Custom|PlayPickupAnim
  ;[1 1 1] Pickup FX Implementation Tick
  (Utilities|FlowControl|Gate true) ; enters at Toggle
)

(event Custom|PickupFX
  (Audio|PlaySound2D (Variables|Default|GetPickupSound) 1.0 1.0 0.0 0 0)
  (CallFunction|PlayPickupAnim))

(event Custom|OnPicked
  (params (Character :type BP%20My%20Character%20Object%20Reference)))

(event EventTick
  (params (DeltaSeconds :type Float%20%28single-precision%29))
  ;[1 1 1] Pickup FX Implementation Tick
  (Utilities|FlowControl|Gate true
    (:Exit
      ;;[1 1 1] get color
      (Variables|Default|SetColorBeforePickup (Math|Conversions|ToColor(LinearColor) (Variables|/Script/Paper2D.PaperSpriteComponent|GetSpriteColor (Variables|Default|GetPaperSprite))))
      ;;[1 1 1] Timer
      (Variables|Default|SetPickupAnimAccomulation (+ (Variables|Default|GetPickupAnimAccomulation) DeltaSeconds))
      (if (>= (Variables|Default|GetPickupAnimAccomulation) (Variables|Default|GetPickupAnimTime))
        (Actor|DestroyActor)
        (else
          ;;[1 1 1] Change Alpha
          (Sprite|SetSpriteColor (Variables|Default|GetPaperSprite) (Utilities|Struct|MakeLinearColor (Math|Conversions|ToFloat(Byte) (.r (Variables|Default|GetColorBeforePickup))) (Math|Conversions|ToFloat(Byte) (.g (Variables|Default|GetColorBeforePickup))) (Math|Conversions|ToFloat(Byte) (.b (Variables|Default|GetColorBeforePickup))) (- 1.0 (/ (Variables|Default|GetPickupAnimAccomulation) (Variables|Default|GetPickupAnimTime))))))))))

(fn ConstructionScript)