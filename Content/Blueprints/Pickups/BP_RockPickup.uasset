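; BP_RockPickup is a sprite-based rock pickup that the player can carry and put down with the Interact input.
; Pickup overlap stores the character, shows a HUD prompt and enables the actor's input; leaving disables input and clears the reference.
; Interact toggles carrying through the character's SetStoneCarry, refusing pickup if a stone is already carried.
; Hard impacts against anything except the player character play a hit sound, unless already playing.
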(event OnComponentHit(PaperSprite)
  (params (HitComponent :type Primitive%20Component%20Object%20Reference) (OtherActor :type Actor%20Object%20Reference) (OtherComp :type Primitive%20Component%20Object%20Reference) (NormalImpulse :type Vector :default "0, 0, 0") (Hit :type Hit%20Result%20Structure%20%28by%20ref%29))
  (bind _hitaudio (Variables|Default|GetHitAudio))
  ;[1 1 1] Hit Sound
  (Utilities|Casting|CastToBP_MyCharacter OtherActor
    (:CastFailed
      (if (> (Math|Vector|VectorLength NormalImpulse) 2e+03)
        (if (not (Audio|Components|Audio|IsPlaying _hitaudio))
          (Audio|Components|Audio|Play _hitaudio 0.0))))))

(event OnComponentEndOverlap(PickupCollision)
  (params (OverlappedComponent :type Primitive%20Component%20Object%20Reference) (OtherActor :type Actor%20Object%20Reference) (OtherComp :type Primitive%20Component%20Object%20Reference) (OtherBodyIndex :type Integer))
  ;[1 1 1] On End Overlap
  (if (== OtherActor (Variables|Default|GetCharacter))
    (CallFunction|DisableCharacterInput)
    (Variables|Default|SetCharacter 0)))

(event EventTick
  (params (DeltaSeconds :type Float%20%28single-precision%29)))

(event EventPlayPickupAnim)

(event EventOnPicked
  (params (Character :type BP%20My%20Character%20Object%20Reference))
  ;[1 1 1] On Overlap
  (bind _output_get (Variables|Default|SetCharacter Character))
  (Utilities|IsValid _output_get
    (:Is%20Valid
      (|HUDPressEToPickStone)
      (CallFunction|EnableCharacterInput))))

(event Input|ActionEvents|InputActionInteract
  (params (Key :type Key%20Structure :default "None"))
  (bind _character (Variables|Default|GetCharacter))
  (bind _character_2 (Variables|Default|GetCharacter))
  ;[1 1 1] Pressed E
  (:Pressed
    (Utilities|IsValid _character_2
      (:Is%20Valid
        (if (Variables|Default|GetbIsCarried)
          (Default|SetStoneCarry _character false 0 false)
          (elif (not (Default|GetIsCarryStone _character_2))
            (Default|SetStoneCarry _character true self false)))))))

(fn ConstructionScript
  (|CallParentFunction))

(fn EnableCharacterInput
  (Utilities|IsValid (Variables|Default|GetCharacter)
    (:Is%20Valid
      (bind _asplayer_controller (Utilities|Casting|CastToPlayerController (Pawn|GetController (Variables|Default|GetCharacter))))
      (Input|EnableInput _asplayer_controller))))

(fn DisableCharacterInput
  (Utilities|IsValid (Variables|Default|GetCharacter)
    (:Is%20Valid
      (bind _asplayer_controller (Utilities|Casting|CastToPlayerController (Pawn|GetController (Variables|Default|GetCharacter))))
      (Input|DisableInput _asplayer_controller))))