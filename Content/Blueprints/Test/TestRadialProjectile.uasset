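; TestRadialProjectile is a test Blueprint that previews a radial spread of points, likely for projectile placement.
; Its construction script adds a static mesh and an arrow component at each of Number points along a vertical arc of given Radius.
; Each point is a downward vector rotated in pitch, splitting Angle into equal segments and using their midpoints, centered on Offset.
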(fn ConstructionScript
  (bind _angle (Variables|Default|GetAngle))
  (bind _number (Variables|Default|GetNumber))
  (bind _returnvalue (Math|Conversions|ToFloat(Integer) _number))
  (bind _returnvalue_2 (/ _angle _returnvalue))
  (for _index (range 0 (- _number 1))
    (AddComponent|AddStaticMeshComponent false (Math|Transform|MakeTransform (Math|Vector|RotateVector (Math|Vector|MakeVector 0.0 0.0 (* (Variables|Default|GetRadius) -1.0)) (Math|Rotator|MakeRotator 0.0 (+ (* _index _returnvalue_2) (Variables|Default|GetOffset) (* (Variables|Default|GetAngle) -0.5) (* _returnvalue_2 0.5)) 0.0)) "0, 0, 0" "1,1,1"))
    (AddComponent|AddArrowComponent false (Math|Transform|MakeTransform (Math|Vector|RotateVector (Math|Vector|MakeVector 0.0 0.0 (* (Variables|Default|GetRadius) -1.0)) (Math|Rotator|MakeRotator 0.0 (+ (* _index _returnvalue_2) (Variables|Default|GetOffset) (* (Variables|Default|GetAngle) -0.5) (* _returnvalue_2 0.5)) 0.0)) (Math|Rotator|MakeRotator 0.0 0.0 0.0) "1,1,1"))))