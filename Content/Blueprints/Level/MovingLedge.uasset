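; Moving ledge actor that carries a sprite between StartPoint and EndPoint like an elevator, pausing at each end before reversing.
; A timeline scaled by MovementRate drives the position lerp.
; A looping timer sphere-traces below the ledge for the player character and plays the timeline forward again if it is reversing.
; The construction script's TestEndPoint toggle previews the end position and snaps the actor to Y=0.
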(event Custom|LookForObstruction
  (bind _movingledgesprite (Variables|Default|GetMovingLedgeSprite))
  (bind _returnvalue (Transformation|GetWorldLocation _movingledgesprite))
  (bind _outhit (Collision|SphereTraceForObjects (- _returnvalue "0, 0,100.000000") (- _returnvalue "0, 0,101.000000") (/ (.SphereRadius (Collision|GetComponentBounds _movingledgesprite)) 2.0) (Utilities|Array|MakeArray "ObjectTypeQuery3") false 0 "None"))
  (Utilities|Casting|CastToBP_MyCharacter (.hitactor _outhit))
  (if (Class|TimelineComponent|IsReversing)
    (CallFunction|ElevatorObstructed)))

(event Custom|ElevatorObstructed
  (bind (_direction _newtrack_0) (Timeline|ElevatorTimeline Play)
    (:Update
      (Transformation|SetRelativeLocation (Variables|Default|GetMovingLedgeSprite) (Math|Vector|Lerp(Vector) (Variables|Default|GetStartPoint) (Variables|Default|GetEndPoint) _newtrack_0) false false))
    (:Finished
      (Utilities|FlowControl|Delay (Variables|Default|GetWaitTime))
      (switch Utilities|FlowControl|Switch|SwitchonETimelineDirection _direction
        (:Forward
          (Timeline|ElevatorTimeline ReverseFromEnd))
        (:Backward
          (Timeline|ElevatorTimeline PlayFromStart))))))

(event EventBeginPlay
  (bind _movementrate (Variables|Default|GetMovementRate))
  (bind _returnvalue (/ 1.0 _movementrate))
  (Components|Timeline|SetPlayRate (Variables|Default|GetElevatorTimeline) _returnvalue)
  (Utilities|Time|SetTimerbyFunctionName 0 "LookForObstruction" _returnvalue true))

(fn ConstructionScript
  (bind _returnvalue (Transformation|GetActorLocation))
  (bind (_x _y _z) (Math|Vector|BreakVector _returnvalue))
  (if (Variables|Default|GetTestEndPoint)
    (Transformation|SetRelativeLocation (Variables|Default|GetMovingLedgeSprite) (Variables|Default|GetEndPoint) false false)
    (Transformation|SetActorLocation (Math|Vector|MakeVector _x 0.0 _z) false false)))