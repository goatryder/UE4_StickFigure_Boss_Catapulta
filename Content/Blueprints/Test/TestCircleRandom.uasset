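; TestCircleRandom is a test Blueprint that scatters static mesh components at random points inside a circle.
; Its construction script adds Number meshes, each placed by a random angle and a random distance up to Radius, converted to relative X and Z offsets in a vertical plane.
; The distance is sampled linearly without square-root correction, so points cluster toward the center.
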(fn ConstructionScript
  (for _index (range 0 (- (Variables|Default|GetNumber) 1))
    (LocalVariables|SetTheta (Math|Float|MultiplybyPi (* (Math|Random|RandomFloat) 2.0)))
    (LocalVariables|SetRandRadius (Math|Random|RandomFloatinRange 0.0 (Variables|Default|GetRadius)))
    (AddComponent|AddStaticMeshComponent false (Math|Transform|MakeTransform (Math|Vector|MakeVector (+ 0.0 (* (LocalVariables|GetRandRadius) (Math|Trig|Cos(Radians) (LocalVariables|GetTheta)))) 0.0 (+ 0.0 (* (Math|Trig|Sin(Radians) (LocalVariables|GetTheta)) (LocalVariables|GetRandRadius)))) "0, 0, 0" "1,1,1"))))