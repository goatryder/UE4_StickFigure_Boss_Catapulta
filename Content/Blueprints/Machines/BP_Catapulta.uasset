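; Player-operated Paper2D catapult that is loaded with a carried stone, aimed and fired, and breaks when an enemy slow projectile overlaps it.
; Overlap tracks the character and updates HUD hints; Interact reloads it or toggles character control, driven by a loaded/fired/broken state.
; Reload spawns a hidden projectile that Fire launches along the aimed velocity.
; While loaded, Tick rebuilds sprite markers along the predicted trajectory every frame.
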(event OnComponentBeginOverlap(InteractCollision)
  (params (OverlappedComponent :type Primitive%20Component%20Object%20Reference) (OtherActor :type Actor%20Object%20Reference) (OtherComp :type Primitive%20Component%20Object%20Reference) (OtherBodyIndex :type Integer) (bFromSweep :type Boolean) (SweepResult :type Hit%20Result%20Structure%20%28by%20ref%29))
  (Utilities|Casting|CastToEnemyProjectileSlow OtherActor
    (:then
      (CallFunction|BreakCatapulta)
      (Collision|SetCollisionResponsetoChannel (Variables|Default|GetInteractCollision) "ECC_GameTraceChannel1" "ECR_Ignore"))
    (:CastFailed
      (bind _asbp_my_character (Utilities|Casting|CastToBP_MyCharacter OtherActor))
      (Variables|Default|SetOverlappingCharacter _asbp_my_character)
      (Utilities|FlowControl|Sequence
        (:then_0
          ;[1 1 1] If Carring Stone Actor Temporary Disable it's Input
          (Utilities|IsValid (Variables|/Game/Blueprints/BP_MyCharacter.BP_MyCharacter_C|GetCarringStone (Variables|Default|GetOverlappingCharacter))
            (:Is%20Valid
              (Default|DisableCharacterInput (Variables|/Game/Blueprints/BP_MyCharacter.BP_MyCharacter_C|GetCarringStone (Variables|Default|GetOverlappingCharacter))))))
        (:then_1
          ;[1 1 1] Add Catapulta Ref To Controller
          (Utilities|IsValid (Variables|/Game/Blueprints/BP_MyCharacter.BP_MyCharacter_C|GetLastController (Variables|Default|GetOverlappingCharacter))
            (:Is%20Valid
              (Variables|/Game/Blueprints/BP_MyConroller.BP_MyConroller_C|SetNearbyCatapulta (Variables|/Game/Blueprints/BP_MyCharacter.BP_MyCharacter_C|GetLastController (Variables|Default|GetOverlappingCharacter)) self))))
        (:then_2
          (CallFunction|HandleHUDMsg))))))

(event OnComponentEndOverlap(InteractCollision)
  (params (OverlappedComponent :type Primitive%20Component%20Object%20Reference) (OtherActor :type Actor%20Object%20Reference) (OtherComp :type Primitive%20Component%20Object%20Reference) (OtherBodyIndex :type Integer))
  (bind _asbp_my_character (Utilities|Casting|CastToBP_MyCharacter OtherActor))
  (if (== _asbp_my_character (Variables|Default|GetOverlappingCharacter))
    (Utilities|FlowControl|Sequence
      (:then_0
        ;[1 1 1] If Carring Stone Actor, Set it's input enabled
        (Utilities|IsValid (Variables|/Game/Blueprints/BP_MyCharacter.BP_MyCharacter_C|GetCarringStone (Variables|Default|GetOverlappingCharacter))
          (:Is%20Valid
            (Default|EnableCharacterInput (Variables|/Game/Blueprints/BP_MyCharacter.BP_MyCharacter_C|GetCarringStone (Variables|Default|GetOverlappingCharacter))))))
      (:then_1
        ;[1 1 1] Clear Controller Catapulta Ref
        (Utilities|IsValid (Variables|/Game/Blueprints/BP_MyCharacter.BP_MyCharacter_C|GetLastController (Variables|Default|GetOverlappingCharacter))
          (:Is%20Valid
            (Variables|/Game/Blueprints/BP_MyConroller.BP_MyConroller_C|SetNearbyCatapulta (Variables|/Game/Blueprints/BP_MyCharacter.BP_MyCharacter_C|GetLastController (Variables|Default|GetOverlappingCharacter)) 0))))
      (:then_2
        (Variables|Default|SetOverlappingCharacter 0)))))

(event Custom|FireCatapulta
  ;[1 1 1] Fire Logic
  (Utilities|IsBroken
    (:False
      (Variables|Default|SetState "NewEnumerator6")
      (Rendering|Components|Sprite|SetSprite (Variables|Default|GetPaperSprite) (Variables|Default|GetSprite_Idle))
      (Audio|PlaySound2D (Variables|Default|GetFireSound) 1.0 1.0 0.0 0 0)
      (CallFunction|ActivateProjectile)
      (Utilities|FlowControl|Delay 5.0)
      (Utilities|CharacterStopUsingCatapulta))))

(event Custom|ReloadCatapulta
  ;[1 1 1] Reload Logic
  (Utilities|IsBroken
    (:False
      (Variables|Default|SetState "NewEnumerator7")
      (Rendering|Components|Sprite|SetSprite (Variables|Default|GetPaperSprite) (Variables|Default|GetSprite_Ready))
      (Audio|PlaySound2D (Variables|Default|GetReloadSound) 1.0 1.0 0.0 0 0)
      (CallFunction|SpawnProjectile)
      (Utilities|CharacterRemoveStone))))

(event Custom|BreakCatapulta
  ;[1 1 1] Break Logic
  (Variables|Default|SetState "NewEnumerator8")
  (Rendering|Components|Sprite|SetSprite (Variables|Default|GetPaperSprite) (Variables|Default|GetSprite_Broken))
  (Audio|PlaySound2D (Variables|Default|GetBreakSound) 1.0 1.0 0.0 0 0)
  (Effects|SpawnEmitteratLocation "/Game/Effects/KillEnemy.KillEnemy" (Transformation|GetWorldLocation (Variables|Default|GetPaperSprite)))
  (Default|CallBrakes))

(event Custom|ActivateProjectile
  (bind _spawnedprojectile (Variables|Default|GetSpawnedProjectile))
  (bind _projectilemovement1 (Variables|/Game/Blueprints/Projectiles/ProjectileBase.ProjectileBase_C|GetProjectileMovement1 _spawnedprojectile))
  ;[1 1 1] Spawn Projectile Logic
  (Utilities|IsValid (Variables|Default|GetSpawnedProjectile)
    (:Is%20Valid
      ;;[1 1 1] Correct Location
      (Transformation|SetActorLocation _spawnedprojectile (Transformation|GetWorldLocation (Variables|Default|GetProjectileSpawnArrow)) false false)
      (Rendering|SetActorHiddenInGame _spawnedprojectile false)
      ;;[1 1 1] Correct Velocity
      (Variables|/Script/Engine.MovementComponent|SetVelocity _projectilemovement1 (* (Variables|Default|GetProjectileVelocity) (Variables|/Script/Engine.ProjectileMovementComponent|GetInitialSpeed _projectilemovement1)))
      (Components|Activation|Activate _projectilemovement1 false))))

(event Custom|InteractScope
  (bind _overlappingcharacter (Variables|Default|GetOverlappingCharacter))
  ;[1 1 1] INPUT Interact
  (Utilities|IsValid _overlappingcharacter
    (:Is%20Valid
      (Utilities|IsLoaded
        (:True
          (Default|SetUsingCatapulta _overlappingcharacter (not (Variables|Default|GetbIsUsedByCharacter)) self))
        (:False
          (Utilities|IsCharacterCarringStone
            (:True
              (CallFunction|ReloadCatapulta)
              (CallFunction|HandleHUDMsg))))))))

(event Custom|AllowToBeDestroyedByProjectile
  (Collision|SetCollisionResponsetoChannel (Variables|Default|GetInteractCollision) "ECC_GameTraceChannel1" "ECR_Overlap"))

(event Custom|SpawnProjectile
  ;[1 1 1] Spawn Projectile Logic
  (bind _returnvalue (Game|SpawnActorfromClass "/Game/Blueprints/Projectiles/CatapultaProjectile.CatapultaProjectile_C" (Math|Transform|MakeTransform (Transformation|GetActorLocation) "0, 0, 0" "1,1,1") "Undefined" 0 0))
  (Variables|Default|SetSpawnedProjectile _returnvalue)
  (Rendering|SetActorHiddenInGame _returnvalue true)
  (Utilities|IsValid _returnvalue
    (:Is%20Valid
      ;;[1 1 1] Projectile Hit Observer
      (Collision|BindEventtoOnActorHit _returnvalue (delegate Custom|ProjectileHitObserved)))))

(event Custom|ProjectileHitObserved
  (params (SelfActor :type Actor%20Object%20Reference) (OtherActor :type Actor%20Object%20Reference) (NormalImpulse :type Vector) (Hit :type Hit%20Result%20Structure%20%28by%20ref%29))
  ;[1 1 1] Spawn Projectile Logic
  ;;[1 1 1] Projectile Hit Observer
  (Utilities|CharacterStopUsingCatapulta))

(event EventPossessed
  (params (NewController :type Controller%20Object%20Reference)))

(event EventUnpossessed
  (params (OldController :type Controller%20Object%20Reference)))

(event EventTick
  (params (DeltaSeconds :type Float%20%28single-precision%29))
  (if (Utilities|Enum|Equal(Enum) (Variables|Default|GetState) "NewEnumerator7")
    (CallFunction|DestroyMarkerSprites)
    (CallFunction|ProjectilePrediction)
    (else
      (CallFunction|DestroyMarkerSprites))))

(event Input|ActionEvents|InputActionFire
  (params (Key :type Key%20Structure :default "None"))
  ;[1 1 1] INPUT Fire
  (:Pressed
    (if (Variables|Default|GetbIsUsedByCharacter)
      (if (Utilities|Enum|Equal(Enum) (Variables|Default|GetState) "NewEnumerator7")
        (CallFunction|FireCatapulta)))))

(event Input|ActionEvents|InputActionInteract
  (params (Key :type Key%20Structure :default "None"))
  ;[1 1 1] INPUT Interact
  (:Pressed
    (CallFunction|InteractScope)))

(event Input|AxisEvents|InputAxisMachineAimVertical
  (params (AxisValue :type Float%20%28single-precision%29))
  ;[1 1 1] INPUT Aim Horizontally
  (CallFunction|AdjustProjectileHorizontalVelocity AxisValue))

(event Input|AxisEvents|InputAxisMoveRight
  (params (AxisValue :type Float%20%28single-precision%29))
  ;[1 1 1] INPUT Aim Vertically
  (CallFunction|RotateonInputRight AxisValue))

(fn ConstructionScript)

(fn HandleHUDMsg
  (Utilities|IsBroken
    (:True
      (|HudCatapultaBroken))
    (:False
      (Utilities|IsLoaded
        (:True
          (|HUDCatapultaControl))
        (:False
          (Utilities|IsCharacterCarringStone
            (:True
              (|HudCatapultaPressEtoLoad))
            (:False
              (|HudCatapultaNeedStone))))))))

(fn RotateonInputRight
  (params (RightVal :type Float%20%28single-precision%29))
  (bind _returnvalue (Pawn|GetController))
  (bind _returnvalue_2 (Pawn|GetController))
  (Math|Float|CompareFloat RightVal 0.0
    (:>
      (Utilities|IsValid _returnvalue_2
        (:Is%20Valid
          (Pawn|SetControlRotation _returnvalue_2 (Math|Rotator|MakeRotator 0.0 0.0 0.0))
          (Variables|Default|SetProjectileVelocity (Math|Vector|Normalize (Math|Vector|MakeVector (* (Math|Float|Absolute(Float) (.x (Variables|Default|GetProjectileVelocity))) -1.0) (.y (Variables|Default|GetProjectileVelocity)) (.z (Variables|Default|GetProjectileVelocity)))))
          (Variables|Default|SetbFlipSide false))))
    (:<
      (Utilities|IsValid _returnvalue
        (:Is%20Valid
          (Pawn|SetControlRotation _returnvalue (Math|Rotator|MakeRotator 0.0 0.0 1.8e+02))
          (Variables|Default|SetProjectileVelocity (Math|Vector|Normalize (Math|Vector|MakeVector (Math|Float|Absolute(Float) (.x (Variables|Default|GetProjectileVelocity))) (.y (Variables|Default|GetProjectileVelocity)) (.z (Variables|Default|GetProjectileVelocity)))))
          (Variables|Default|SetbFlipSide true))))))

(fn ProjectilePrediction
  (bind _spawnedprojectile (Variables|Default|GetSpawnedProjectile))
  (bind _projectilemovement1 (Variables|/Game/Blueprints/Projectiles/ProjectileBase.ProjectileBase_C|GetProjectileMovement1 _spawnedprojectile))
  (Utilities|IsValid _spawnedprojectile
    (:Is%20Valid
      (bind _predictresult (Class|GameplayStatics|BlueprintPredictProjectilePathAdvanced (Utilities|Struct|MakePredictProjectilePathParams (Transformation|GetWorldLocation (Variables|Default|GetProjectileSpawnArrow)) (* (Variables|Default|GetProjectileVelocity) (Variables|/Script/Engine.ProjectileMovementComponent|GetInitialSpeed _projectilemovement1)) true (Variables|/Script/Engine.SphereComponent|GetSphereRadius (Variables|/Game/Blueprints/Projectiles/ProjectileBase.ProjectileBase_C|GetCollision _spawnedprojectile)) 4.0 true "ECC_GameTraceChannel3" "ObjectTypeQuery1" 0 1e+01 (Components|Movement|GetGravityZ _projectilemovement1) "None" 0.1 false)))
      (for _array_element (.pathdata _predictresult)
        (bind _returnvalue (AddComponent|AddPaperSpriteComponent false))
        (Transformation|SetWorldTransform _returnvalue (Math|Transform|MakeTransform (.location _array_element) (Math|Rotator|MakeRotator 0.0 (* (Class|KismetMathLibrary|DegAcos (Math|Vector|DotProduct (Math|Vector|Normalize (.velocity _array_element)) "0.000000, 0,1.000000")) (Math|Float|Sign(Float) (Math|Vector|DotProduct (Math|Vector|CrossProduct (Math|Vector|Normalize (.velocity _array_element)) "0.000000, 0,1.000000") "0,1.000000, 0"))) 0.0) "1,1,1") false false)
        (Utilities|Array|Add (Variables|Default|GetMarkerSprites) _returnvalue)))))

(fn AdjustProjectileHorizontalVelocity
  (params (InputVal :type Float%20%28single-precision%29))
  (if (Variables|Default|GetbFlipSide)
    (Variables|Default|SetProjectileVelocity (Math|Vector|Normalize (Math|Vector|MakeVector (Math|Float|Clamp(Float) (.x (Math|Vector|RotateVector (Variables|Default|GetProjectileVelocity) (Math|Rotator|MakeRotator 0.0 InputVal 0.0)))) (.y (Math|Vector|RotateVector (Variables|Default|GetProjectileVelocity) (Math|Rotator|MakeRotator 0.0 InputVal 0.0))) (Math|Float|Clamp(Float) (.z (Math|Vector|RotateVector (Variables|Default|GetProjectileVelocity) (Math|Rotator|MakeRotator 0.0 InputVal 0.0)))))))
    (else
      (Variables|Default|SetProjectileVelocity (Math|Vector|Normalize (Math|Vector|MakeVector (Math|Float|Clamp(Float) (.x (Math|Vector|RotateVector (Variables|Default|GetProjectileVelocity) (Math|Rotator|MakeRotator 0.0 InputVal 0.0))) -1.0 0.0) (.y (Math|Vector|RotateVector (Variables|Default|GetProjectileVelocity) (Math|Rotator|MakeRotator 0.0 InputVal 0.0))) (Math|Float|Clamp(Float) (.z (Math|Vector|RotateVector (Variables|Default|GetProjectileVelocity) (Math|Rotator|MakeRotator 0.0 InputVal 0.0))))))))))

(fn DestroyMarkerSprites
  (for _array_element (Variables|Default|GetMarkerSprites)
    (Utilities|IsValid _array_element
      (:Is%20Valid
        (Components|DestroyComponent _array_element))))
  (Utilities|Array|Clear (Variables|Default|GetMarkerSprites)))