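; Catapult projectile that spins its flipbook sprite in flight and damages enemy armour and health on impact.
; When movement activates, it reverses spin for negative X velocity and activates its spawned emitter if valid.
; Hits on the player character are ignored; any other hit triggers an overridden FX event that spawns a collide actor and plays a sound, then the projectile destroys itself.
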(event OnComponentHit(Collision)
  (params (HitComponent :type Primitive%20Component%20Object%20Reference) (OtherActor :type Actor%20Object%20Reference) (OtherComp :type Primitive%20Component%20Object%20Reference) (NormalImpulse :type Vector :default "0, 0, 0") (Hit :type Hit%20Result%20Structure%20%28by%20ref%29))
  (Utilities|Casting|CastToBP_MyCharacter OtherActor
    (:CastFailed
      (CallFunction|CollidedFX)
      (bind _asenemy (Utilities|Casting|CastToEnemy OtherActor)
        (:then
          (Default|DamageArmour _asenemy (Variables|Default|GetArmourDamageAmount))
          (Default|DamageHealth _asenemy (Variables|Default|GetHealthDamageAmount)))
        (:CastFailed
          _))
      (Actor|DestroyActor))))

(event OnComponentActivated(ProjectileMovement1)
  (params (Component :type Actor%20Component%20Object%20Reference) (bReset :type Boolean))
  (bind _spawnedemitter (Variables|Default|GetSpawnedEmitter))
  ;[1 1 1] If Abs projectile X velocity is negative, rotate in opposite direction
  (Math|Float|CompareFloat (.x (Variables|/Script/Engine.MovementComponent|GetVelocity (Variables|Default|GetProjectileMovement1))) 0.0
    (:>
      _)
    (:==
      _)
    (:<
      (Variables|Default|SetRotateRate (* (Variables|Default|GetRotateRate) -1.0))))
  (Utilities|IsValid _spawnedemitter
    (:Is%20Valid
      (Components|Activation|Activate _spawnedemitter false))))

(event EventCollidedFX
  ;[1 1 1] Collide Fx Override
  (Game|SpawnActorfromClass (Variables|Default|GetCollideActorSpawn) (Math|Conversions|ToTransform(Vector) (Transformation|GetActorLocation)) "AdjustIfPossibleButDontSpawnIfColliding" 0 0)
  (Audio|PlaySoundatLocation (Variables|Default|GetCollideSound) (Transformation|GetActorLocation) "0, 0, 0" 2.0 0.7 0.0 "/Game/Sound/CatapultaRockAttenuation.CatapultaRockAttenuation" 0 0))

(event EventTick
  (params (DeltaSeconds :type Float%20%28single-precision%29))
  ;[1 1 1] Rotate Sprite
  (Transformation|AddLocalRotation (Variables|Default|GetPaperFlipbook) (Math|Rotator|MakeRotator 0.0 (* DeltaSeconds (Variables|Default|GetRotateRate)) 0.0) false false))

(fn ConstructionScript
  (|CallParentFunction))