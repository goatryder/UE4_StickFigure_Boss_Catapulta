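; A chaotic player projectile that flies with randomised speed, arc and direction, damaging enemies it hits.
; On spawn it picks a random low gravity scale, then scales its X and Z velocity by separate random factors and zeroes Y, keeping flight in the XZ plane.
; Collisions ignore the player character; any other actor destroys the projectile, with enemies first taking armour and health damage.
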(event EventCollided
  (params (Actor :type Actor%20Object%20Reference))
  (Utilities|Casting|CastToBP_MyCharacter Actor
    (:CastFailed
      (bind _asenemy (Utilities|Casting|CastToEnemy Actor)
        (:then
          (Default|DamageArmour _asenemy (Variables|Default|GetArmourDamageAmount))
          (Default|DamageHealth _asenemy (Variables|Default|GetHealthDamageAmount)))
        (:CastFailed
          _))
      (Actor|DestroyActor))))

(event EventBeginPlay
  (|CallParentFunction)
  (Variables|/Script/Engine.ProjectileMovementComponent|SetProjectileGravityScale (Variables|Default|GetProjectileMovement1) (Math|Random|RandomFloatinRange 0.05 0.22))
  (CallFunction|ChangeVelocity))

(fn ConstructionScript
  (|CallParentFunction))

(fn ChangeVelocity
  (bind _projectilemovement1 (Variables|Default|GetProjectileMovement1))
  (Variables|/Script/Engine.MovementComponent|SetVelocity _projectilemovement1 (Math|Vector|MakeVector (* (.x (Variables|/Script/Engine.MovementComponent|GetVelocity _projectilemovement1)) (Math|Random|RandomFloatinRange 0.8 1.1)) 0.0 (* (.z (Variables|/Script/Engine.MovementComponent|GetVelocity _projectilemovement1)) (Math|Random|RandomFloatinRange 0.7 1.3)))))