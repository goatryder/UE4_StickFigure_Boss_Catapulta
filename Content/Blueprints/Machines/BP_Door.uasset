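; A locked sliding door that a character unlocks by spending a key, then opens and closes by proximity.
; On overlap it shows a HUD use-key or find-key prompt and enables interact input if keys are held.
; Using a key plays a sound, and the door opens when that audio finishes.
; Timelines slide the sprite by an offset, rechecking overlap on completion to reverse if needed.
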(event OnComponentBeginOverlap(InterractCollision)
  (params (OverlappedComponent :type Primitive%20Component%20Object%20Reference) (OtherActor :type Actor%20Object%20Reference) (OtherComp :type Primitive%20Component%20Object%20Reference) (OtherBodyIndex :type Integer) (bFromSweep :type Boolean) (SweepResult :type Hit%20Result%20Structure%20%28by%20ref%29))
  ;[1 1 1] Overlap Door
  (bind _asmy_character (Utilities|Casting|CastToBP_MyCharacter OtherActor))
  (Variables|Default|SetCharacterNearDoor _asmy_character)
  (Variables|Default|SetbCanOpen true)
  (if (Variables|Default|GetbKeyUsed)
    (CallFunction|OpenDoor)
    (elif (> (Variables|/Game/Blueprints/BP_MyCharacter.BP_MyCharacter_C|GetKeyNum _asmy_character) 0)
      ;;[1 1 1] Input Enable
      (bind _asplayer_controller (Utilities|Casting|CastToPlayerController (Pawn|GetController (Variables|Default|GetCharacterNearDoor))))
      (Input|EnableInput _asplayer_controller)
      ;;[1 1 1] Hud use key msg
      (bind _asplayer_controller_2 (Utilities|Casting|CastToPlayerController (Pawn|GetController (Variables|Default|GetCharacterNearDoor))))
      (bind _asbp_hud (Utilities|Casting|CastToBP_HUD (HUD|GetHUD _asplayer_controller_2)))
      (Default|UseKeyInfo _asbp_hud)
      (else
        ;;[1 1 1] Hud Find key msg
        (bind _asplayer_controller_3 (Utilities|Casting|CastToPlayerController (Pawn|GetController (Variables|Default|GetCharacterNearDoor))))
        (bind _asbp_hud_2 (Utilities|Casting|CastToBP_HUD (HUD|GetHUD _asplayer_controller_3)))
        (Default|FindKeyInfo _asbp_hud_2)))))

(event OnComponentEndOverlap(InterractCollision)
  (params (OverlappedComponent :type Primitive%20Component%20Object%20Reference) (OtherActor :type Actor%20Object%20Reference) (OtherComp :type Primitive%20Component%20Object%20Reference) (OtherBodyIndex :type Integer))
  ;[1 1 1] End Overlap Door
  (Utilities|Casting|CastToBP_MyCharacter OtherActor)
  (Variables|Default|SetbCanOpen false)
  (CallFunction|CloseDoor))

(event OnAudioFinished(KeyUseAudio)
  ;[1 1 1] Use Key
  (CallFunction|OpenDoor))

(event Custom|CloseDoor
  ;[1 1 1] Close Door
  (if (Variables|Default|GetIsOpen)
    (if (not (Variables|Default|GetbInProgress))
      (Variables|Default|SetbInProgress true)
      (Audio|Components|Audio|Play (Variables|Default|GetOpenAudio) 0.0)
      (bind _openprogress (Timeline|DoorCloseInterpolation PlayFromStart)
        (:Update
          (Transformation|SetRelativeLocation (Variables|Default|GetPaperSprite) (+ (* (Variables|Default|GetDoorOpenOffset) (* _openprogress -1.0)) (Variables|Default|GetDoorInitLocation) (Variables|Default|GetDoorOpenOffset)) false false))
        (:Finished
          (Variables|Default|SetIsOpen false)
          (Variables|Default|SetbInProgress false)
          (if (Variables|Default|GetbCanOpen)
            (CallFunction|OpenDoor)))))))

(event Custom|OpenDoor
  ;[1 1 1] Open Door
  (if (and (Variables|Default|GetbKeyUsed) (not (Variables|Default|GetIsOpen)))
    (if (not (Variables|Default|GetbInProgress))
      (Variables|Default|SetbInProgress true)
      (Audio|Components|Audio|Play (Variables|Default|GetOpenAudio) 0.0)
      (bind _openprogress (Timeline|DoorOpenInterpolation PlayFromStart)
        (:Update
          (Transformation|SetRelativeLocation (Variables|Default|GetPaperSprite) (+ (* (Variables|Default|GetDoorOpenOffset) _openprogress) (Variables|Default|GetDoorInitLocation)) false false))
        (:Finished
          (Variables|Default|SetIsOpen true)
          (Variables|Default|SetbInProgress false)
          (if (not (Variables|Default|GetbCanOpen))
            (CallFunction|CloseDoor)))))))

(event EventBeginPlay
  ;[1 1 1] Get Initial Door Location
  (Variables|Default|SetDoorInitLocation (Variables|/Script/Engine.SceneComponent|GetRelativeLocation (Variables|Default|GetPaperSprite))))

(event Input|ActionEvents|InputActionInteract
  (params (Key :type Key%20Structure))
  ;[1 1 1] Use Key
  (:Pressed
    (if (Math|Boolean|ANDBoolean (Variables|Default|GetbCanOpen) (not (Variables|Default|GetbKeyUsed)) (> (Variables|/Game/Blueprints/BP_MyCharacter.BP_MyCharacter_C|GetKeyNum (Variables|Default|GetCharacterNearDoor)) 0))
      (Audio|Components|Audio|Play (Variables|Default|GetKeyUseAudio) 0.0)
      (Math|Integer|DecrementInt (Variables|/Game/Blueprints/BP_MyCharacter.BP_MyCharacter_C|GetKeyNum (Variables|Default|GetCharacterNearDoor))
        (:%20%20
          (Variables|Default|SetbKeyUsed true)
          ;;[1 1 1] Input Disable
          (bind _asplayer_controller (Utilities|Casting|CastToPlayerController (Pawn|GetController (Variables|Default|GetCharacterNearDoor))))
          (Input|DisableInput _asplayer_controller))))))

(fn ConstructionScript)