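; SteveTheBadguy is an enemy that fires projectile fans at the player and drops a key on death.
; Tick re-aims the fan's pitch at the player, retargeted on respawn via the game mode, and Fire spawns it around that angle.
; When armour breaks, it makes the first catapult found destructible and suspends radial fire.
; It then shoots slow projectiles at that catapult, paced by a Delay, until it breaks.
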(event Custom|ResetCharacterTarget
  (params (RespawnedPlayer :type BP%20My%20Character%20Object%20Reference))
  ;[1 1 1] Reset Target Character On Death
  (Variables|Default|SetTargetCharacter RespawnedPlayer))

(event Custom|ClearTargetCatapulta
  ;[1 1 1] Set Target Catapulta to break
  (Variables|Default|SetTargetCatapulta 0))

(event Custom|TryToDestroyCatapulta
  (Utilities|FlowControl|Delay 2.0)
  (Utilities|IsValid (Variables|Default|GetTargetCatapulta)
    (:Is%20Valid
      (Game|SpawnActorfromClass "/Game/Blueprints/Projectiles/EnemyProjectileSlow.EnemyProjectileSlow_C" (Math|Transform|MakeTransform (Transformation|GetActorLocation) (Math|Rotator|MakeRotationfromAxes (Math|Vector|Normalize (- (Transformation|GetWorldLocation (Variables|/Game/Blueprints/Machines/BP_Catapulta.BP_Catapulta_C|GetCharacterAttachArrow (Variables|Default|GetTargetCatapulta))) (Transformation|GetActorLocation))) "0, 0, 0" "0, 0, 0") "1,1,1") "Undefined" 0 0)
      (Development|PrintString "AIM PROJECTILE AT CATAPUILTA 
" true true "(R=1.000000,G=0.495285,B=0.006423,A=1.000000)"))))

(event EventTick
  (params (DeltaSeconds :type Float%20%28single-precision%29))
  (|CallParentFunction DeltaSeconds)
  (if (Utilities|IsValid (Variables|Default|GetTargetCatapulta))
    (CallFunction|TrytoDestroyCatapulta)
    (else
      (CallFunction|SetAimonCharacterOffset))))

(event EventOnDeath
  (Game|SpawnActorfromClass "/Game/Blueprints/Pickups/BP_Key.BP_Key_C" (Math|Transform|MakeTransform (Transformation|GetActorLocation) "0, 0, 0" "1,1,1") "Undefined" 0 0))

(event EventArmourDestroyed
  (bind _targetcatapulta (Variables|Default|GetTargetCatapulta))
  (Audio|PlaySound2D "/Game/Sound/CrateBreakCue.CrateBreakCue" 3.0 1.0 0.0 0 0)
  ;[1 1 1] Set Target Catapulta to break
  (CallFunction|SetTargetCatapulta)
  (Utilities|IsValid _targetcatapulta
    (:Is%20Valid
      (EventDispatchers|BindEventtoBrakes _targetcatapulta (delegate Custom|ClearTargetCatapulta)))))

(event EventFire
  (Utilities|IsValid (Variables|Default|GetTargetCatapulta)
    (:Is%20Not%20Valid
      (CallFunction|RadialSpawnProjectile))))

(event EventBeginPlay
  (|CallParentFunction)
  (Utilities|FlowControl|Sequence
    (:then_1
      ;[1 1 1] Init Target Character
      (bind _asbp_my_character (Utilities|Casting|CastToBP_MyCharacter (Pawn|GetControlledPawn (Game|GetPlayerController 0))))
      (Variables|Default|SetTargetCharacter _asbp_my_character))
    (:then_2
      ;[1 1 1] Reset Target Character On Death
      (bind _asbp_my_game_mode (Utilities|Casting|CastToBP_MyGameMode (Game|GetGameMode)))
      (EventDispatchers|BindEventtoPlayerRespawned _asbp_my_game_mode (delegate Custom|ResetCharacterTarget)))))

(fn ConstructionScript
  (|CallParentFunction))

(fn RadialSpawnProjectile
  (bind _projectilesangle (Variables|Default|GetProjectilesAngle))
  (bind _projectilesnum (Variables|Default|GetProjectilesNum))
  (bind _returnvalue (Math|Conversions|ToFloat(Integer) _projectilesnum))
  (bind _returnvalue_2 (/ _projectilesangle _returnvalue))
  (for _index (range 0 (- _projectilesnum 1))
    (Game|SpawnActorfromClass "/Game/Blueprints/Projectiles/EnemyRadialProjectile.EnemyRadialProjectile_C" (Math|Transform|MakeTransform (+ (Transformation|GetActorLocation) (Math|Vector|RotateVector (Math|Vector|MakeVector 0.0 0.0 (* (Variables|Default|GetProjectilesRadius) -1.0)) (Math|Rotator|MakeRotator 0.0 (+ (* _index _returnvalue_2) (Variables|Default|GetProjectilesOffset) (* (Variables|Default|GetProjectilesAngle) -0.5) (* _returnvalue_2 0.5)) 0.0))) (Math|Rotator|MakeRotator 0.0 (- (+ (* _index _returnvalue_2) (Variables|Default|GetProjectilesOffset) (* (Variables|Default|GetProjectilesAngle) -0.5) (* _returnvalue_2 0.5)) 9e+01) 0.0) "1,1,1") "Undefined" 0 0)))

(fn SetAimonCharacterOffset
  (bind _returnvalue (Transformation|GetActorLocation))
  (bind _targetcharacter (Variables|Default|GetTargetCharacter))
  (bind _returnvalue_2 (Transformation|GetActorLocation _targetcharacter))
  (bind _returnvalue_3 (- _returnvalue_2 _returnvalue))
  (bind _returnvalue_4 (Math|Vector|Normalize _returnvalue_3))
  (Utilities|IsValid _targetcharacter
    (:Is%20Valid
      (Variables|Default|SetProjectilesOffset (* (Class|KismetMathLibrary|DegAcos (Math|Vector|DotProduct _returnvalue_4 "0,0.000000,-1.000000")) (Math|Float|Sign(Float) (Math|Vector|DotProduct (Math|Vector|CrossProduct _returnvalue_4 "0, 0,-1.000000") "0,1.000000, 0")))))))

(fn SetTargetCatapulta
  (bind _outactors (Actor|GetAllActorsOfClass "/Game/Blueprints/Machines/BP_Catapulta.BP_Catapulta_C"))
  (if (> (Utilities|Array|Length _outactors) 0)
    (bind _output_get (Variables|Default|SetTargetCatapulta (Utilities|Array|Get(acopy) _outactors)))
    (Default|AllowtobeDestroyedbyProjectile _output_get)))