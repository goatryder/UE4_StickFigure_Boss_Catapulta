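; Game mode that handles player respawning, boss fights and level completion.
; Respawn spawns and possesses a new BP_MyCharacter at the last checkpoint, or the first PlayerStart if none, then relinks the HUD.
; Spawned bosses get HUD health widgets; their destruction plus reaching the last checkpoint shows the level-complete widget.
; Restart reloads the current level, as does Next Level, still marked TODO.
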(event Custom|QuitHandle
  (Game|QuitGame 0 "Quit" false))

(event Custom|NextLevelHandle
  (Development|PrintString "GM NextLevelHandle TODO" true true "(R=1.000000,G=0.000000,B=0.000000,A=1.000000)")
  (Variables|Default|SetbIsBossDefeated false)
  (Variables|Default|SetbLastCheckpointReached false)
  (bind _returnvalue (Game|GetCurrentLevelName true))
  (Game|OpenLevel(byName) (Utilities|String|StringToName _returnvalue))
  ;[1 1 1] Hide Level Complete Widget For players
  (for _array_element (Variables|Default|GetPlayerControllers)
    (bind _asbp_hud (Utilities|Casting|CastToBP_HUD (HUD|GetHUD _array_element)))
    (Default|HideLevelCompleteWidget _asbp_hud)))

(event Custom|RestartHandle
  (Variables|Default|SetbIsBossDefeated false)
  (Variables|Default|SetbLastCheckpointReached false)
  (bind _returnvalue (Game|GetCurrentLevelName true))
  (Game|OpenLevel(byName) (Utilities|String|StringToName _returnvalue))
  ;[1 1 1] Hide Level Complete Widget For players
  (for _array_element (Variables|Default|GetPlayerControllers)
    (bind _asbp_hud (Utilities|Casting|CastToBP_HUD (HUD|GetHUD _array_element)))
    (Default|HideLevelCompleteWidget _asbp_hud)))

(event Custom|RespawnCharacter
  (bind _returnvalue (Game|GetPlayerController 0))
  (bind _returnvalue_2 (Game|GetPlayerController 0))
  ;[1 1 1] Any CheckPoint Reached?
  (if (== (Math|Vector|VectorLength (Variables|Default|GetCharacterLastCheckPoint)) 0.0)
    ;[1 1 1] Spawn From First PlayerStart
    (bind _outactors (Actor|GetAllActorsOfClass "/Script/Engine.PlayerStart"))
    (bind _returnvalue_3 (Game|SpawnActorfromClass "/Game/Blueprints/BP_MyCharacter.BP_MyCharacter_C" (Math|Conversions|ToTransform(Vector) (Transformation|GetActorLocation (Utilities|Array|Get(acopy) _outactors))) "AdjustIfPossibleButDontSpawnIfColliding" 0 0))
    (Pawn|Possess _returnvalue _returnvalue_3)
    (bind _asbp_hud (Utilities|Casting|CastToBP_HUD (HUD|GetHUD _returnvalue)))
    (Variables|/Game/Blueprints/BP_HUD.BP_HUD_C|SetCharacter _asbp_hud _returnvalue_3)
    (Default|CallPlayerRespawned _returnvalue_3)
    (else
      ;[1 1 1] SpawnFromCheckPoint
      (bind _returnvalue_4 (Game|SpawnActorfromClass "/Game/Blueprints/BP_MyCharacter.BP_MyCharacter_C" (Math|Transform|MakeTransform (Variables|Default|GetCharacterLastCheckPoint) "0, 0, 0" "1,1,1") "AlwaysSpawn" 0 0))
      (Pawn|Possess _returnvalue_2 _returnvalue_4)
      (bind _asbp_hud_2 (Utilities|Casting|CastToBP_HUD (HUD|GetHUD _returnvalue_2)))
      (Variables|/Game/Blueprints/BP_HUD.BP_HUD_C|SetCharacter _asbp_hud_2 _returnvalue_4)
      (Default|CallPlayerRespawned _returnvalue_4))))

(event Custom|CheckCurrentLevelComplete
  (if (and (Variables|Default|GetbLastCheckpointReached) (Variables|Default|GetbIsBossDefeated))
    ;[1 1 1] Show Level Complete Widget For players
    (for _array_element (Variables|Default|GetPlayerControllers)
      (bind _asbp_hud (Utilities|Casting|CastToBP_HUD (HUD|GetHUD _array_element)))
      (Default|ShowLevelCompleteWidget _asbp_hud))))

(event Custom|BossSpawn
  (params (SpawnLocation :type Vector) (Enemy :type Enemy%20Class%20Reference))
  (if (!= Enemy 0)
    (bind _returnvalue (Game|SpawnActorfromClass Enemy (Math|Transform|MakeTransform SpawnLocation "0, 0, 0" "1,1,1") "AlwaysSpawn" 0 0))
    (Game|BindEventtoOnDestroyed _returnvalue (delegate Custom|BossDefeated))
    (for _array_element (Variables|Default|GetPlayerControllers)
      (bind _asbp_hud (Utilities|Casting|CastToBP_HUD (HUD|GetHUD _array_element)))
      (Default|EventCreateBossHealthWidget _asbp_hud _returnvalue))))

(event Custom|BossDefeated
  (params (DestroyedActor :type Actor%20Object%20Reference))
  (Development|PrintString "GM Boss Defeated" true true "(R=1.000000,G=0.000000,B=0.000000,A=1.000000)" 5.0)
  (Variables|Default|SetbIsBossDefeated true)
  (CallFunction|CheckCurrentLevelComplete))

(event EventBeginPlay
  (bind _outactors (Actor|GetAllActorsOfClass "/Script/Engine.PlayerController"))
  (Variables|Default|SetPlayerControllers _outactors))

(fn ConstructionScript)